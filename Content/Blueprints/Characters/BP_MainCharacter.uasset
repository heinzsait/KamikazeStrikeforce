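; Main character Blueprint that handles the sniper scope overlay shown to the player.
; ShowSniperScope lazily creates and caches a WBP_SniperScope widget, then plays its zoom animation forward or reversed with matching zoom-in or zoom-out sounds.
; An unconnected chain would set the pickup widget's text from the controller's PlayerAvatar on authority, but never runs; Tick and the construction script are empty.
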(event EventShowSniperScope
  (params (show :type Boolean))
  (Utilities|IsValid (Variables|Default|GetSniperWidget)
    (:Is%20Valid
      _)
    (:Is%20Not%20Valid
      (bind _returnvalue (UserInterface|CreateWidget "/Game/Blueprints/HUD/WBP_SniperScope.WBP_SniperScope_C"))
      (UserInterface|Viewport|AddtoViewport _returnvalue 0)
      (Variables|Default|SetSniperWidget _returnvalue)))
  (if show
    (Utilities|IsValid (Variables|Default|GetSniperWidget)
      (:Is%20Valid
        (UserInterface|Animation|PlayAnimation (Variables|Default|GetSniperWidget) (Variables|/Game/Blueprints/HUD/WBP_SniperScope.WBP_SniperScope_C|GetScopeZoomin (Variables|Default|GetSniperWidget)) 0.0 1 "Forward" 1.0 false)
        (Audio|PlaySound2D "/Game/Assets/MilitaryWeapSilver/Sound/SniperRifle/Cues/SniperRifle_ZoomIn_Cue.SniperRifle_ZoomIn_Cue" 1.0 1.0 0.0 0 0)))
    (else
      (Utilities|IsValid (Variables|Default|GetSniperWidget)
        (:Is%20Valid
          (UserInterface|Animation|PlayAnimation (Variables|Default|GetSniperWidget) (Variables|/Game/Blueprints/HUD/WBP_SniperScope.WBP_SniperScope_C|GetScopeZoomin (Variables|Default|GetSniperWidget)) 0.0 1 "Reverse" 1.0 false)
          (Audio|PlaySound2D "/Game/Assets/MilitaryWeapSilver/Sound/SniperRifle/Cues/SniperRifle_ZoomOut_Cue.SniperRifle_ZoomOut_Cue" 1.0 1.0 0.0 0 0))))))

(event EventTick
  (params (DeltaSeconds :type Float%20%28single-precision%29)))

(fn ConstructionScript)